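; Debris barrel physics prop that reacts to wind, can catch fire, and supports level-style reset.
; Wind pushes it only when lying on its side, strongly favoring force perpendicular to its axis so it rolls.
; Catching fire toggles the particle effect and adds or removes a FireComponent fed by mesh hits.
; It registers as windable and resetable; reset restores the starting transform, kills velocity and extinguishes it.
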(event EventBeginPlay
  (|CallParentFunction)
  (Class|TWABlueprintLibrary|RegisterWindable)
  (Class|TWABlueprintLibrary|RegisterResetable)
  (Variables|Default|SetInitialTransform (Transformation|GetActorTransform)))

(event EventWind
  (params (windForce :type Vector%20%28by%20ref%29 :default "0, 0, 0"))
  (if (< (Math|Float|Absolute(Float) (.z (Math|Vector|GetUpVector (Variables|Default|GetMesh)))) 0.35)
    (Class|TWABlueprintLibrary|SimplePhysicsWind 0 (* windForce 4.0 (Math|Float|Power (Math|Float|Absolute(Float) (Math|Vector|DotProduct windForce (Math|Vector|CrossProduct (Math|Vector|GetUpVector (Variables|Default|GetMesh)) "0.000000,0.000000,1.000000"))) 3.0)) 3.0)))

(event EventExtinguish
  (CallFunction|SetonFire false))

(event EventEndPlay
  (params (EndPlayReason :type EEndPlayReason%20Enum :default "Destroyed"))
  (|CallParentFunction EndPlayReason)
  (Class|TWABlueprintLibrary|RegisterWindable)
  (Class|TWABlueprintLibrary|UnregisterResetable))

(event EventCatchFire
  (CallFunction|SetonFire true))

(event EventReset
  (Transformation|SetActorTransform (Variables|Default|GetInitialTransform))
  (Class|TWABlueprintLibrary|KillVelocity self)
  (if (Class|Flammable|IsFlaming)
    (Class|Flammable|Extinguish)))

(fn ConstructionScript)

(fn SetonFire
  (params (OnFire :type Boolean))
  (bind _returnvalue (Actor|GetComponentbyClass "/Script/GGJ.FireComponent"))
  (bind _p_fire (Variables|Default|GetP_Fire))
  (bind _output_get (Variables|Default|SetOnFire OnFire))
  (if _output_get
    (Components|Activation|Activate _p_fire false)
    (Utilities|IsValid _returnvalue
      (:Is%20Not%20Valid
        (bind _returnvalue_2 (Game|AddComponentbyClass "/Script/GGJ.FireComponent"))
        (Class|FireComponent|DelegateComponentHit _returnvalue_2 (Variables|Default|GetMesh))))
    (else
      (Components|Activation|Deactivate _p_fire)
      (Utilities|IsValid _returnvalue
        (:Is%20Valid
          (Components|DestroyComponent _returnvalue))))))

(fn RefreshFireScale)

(fn GetZLimit
  (return ""))

(fn IsFlaming
  (bind _returnvalue (Class|TWABlueprintLibrary|DefaultIsFlaming))
  (return (or _returnvalue (Variables|Default|GetOnFire))))