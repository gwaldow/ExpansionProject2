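; Resettable cow actor that moos on a repeating timeline, eats non-flaming tumbleweeds and backs away from burning objects.
; EatBox overlaps pull tumbleweeds in and kill them during the eat animation, while SenseBox checks the Flammable interface to trigger short moves along its forward axis.
; Tick drives swept movement with stuck detection, timelines animate the scene component for walking and eating, and collisions shove barrels away.
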(event OnComponentBeginOverlap(SenseBox)
  (params (OverlappedComponent :type Primitive%20Component%20Object%20Reference) (OtherActor :type Actor%20Object%20Reference) (OtherComp :type Primitive%20Component%20Object%20Reference) (OtherBodyIndex :type Integer) (bFromSweep :type Boolean) (SweepResult :type Hit%20Result%20Structure%20%28by%20ref%29))
  (CallFunction|CheckforSense))

(event OnComponentBeginOverlap(EatBox)
  (params (OverlappedComponent :type Primitive%20Component%20Object%20Reference) (OtherActor :type Actor%20Object%20Reference) (OtherComp :type Primitive%20Component%20Object%20Reference) (OtherBodyIndex :type Integer) (bFromSweep :type Boolean) (SweepResult :type Hit%20Result%20Structure%20%28by%20ref%29))
  (bind _astumble_weed_bp (Utilities|Casting|CastToTumbleWeed_BP OtherActor))
  (if (not (Class|Flammable|IsFlaming _astumble_weed_bp))
    (Default|SetForcedLocation _astumble_weed_bp (Transformation|GetWorldLocation (Variables|Default|GetEatBox)))
    (CallFunction|Eat)
    (Audio|SpawnSoundatLocation "/Game/Audio/Cues/CowEat_Cue.CowEat_Cue" (Transformation|GetActorLocation) "0, 0, 0" 1.0 1.0 0.0 0 0)))

(event OnComponentHit(CowCollision)
  (params (HitComponent :type Primitive%20Component%20Object%20Reference) (OtherActor :type Actor%20Object%20Reference) (OtherComp :type Primitive%20Component%20Object%20Reference) (NormalImpulse :type Vector :default "0, 0, 0") (Hit :type Hit%20Result%20Structure%20%28by%20ref%29))
  (bind _returnvalue (Transformation|GetActorLocation))
  (bind _returnvalue_2 (Transformation|GetActorLocation OtherActor))
  (bind _returnvalue_3 (- _returnvalue_2 _returnvalue))
  (bind _returnvalue_4 (Math|Vector|Normalize _returnvalue_3))
  (bind _returnvalue_5 (* _returnvalue_4 1.1e+03))
  (bind _asdebris_barrel_bp (Utilities|Casting|CastToDebris_Barrel_BP OtherActor)
    (:then
      (Physics|AddImpulse (Variables|/Game/GameObjects/Debris_Barrel_BP.Debris_Barrel_BP_C|GetMesh _asdebris_barrel_bp) _returnvalue_5 "None" false))
    (:CastFailed
      (bind _asmetal_barrel_bp (Utilities|Casting|CastToMetal_Barrel_BP OtherActor))
      (Physics|AddImpulse (Variables|/Game/GameObjects/Metal_Barrel_BP.Metal_Barrel_BP_C|GetMesh _asmetal_barrel_bp) _returnvalue_5 "None" false))))

(event Custom|Eat
  (bind _scene (Variables|Default|GetScene))
  (bind _relativerotation (Variables|/Script/Engine.SceneComponent|GetRelativeRotation _scene))
  (if (not (Audio|Components|Audio|IsPlaying (Variables|Default|GetEat_Timeline)))
    (bind (_direction _scale _pitch) (Timeline|Eat_Timeline PlayFromStart)
      (:Update
        (Transformation|SetRelativeScale3D _scene (Math|Vector|MakeVector _scale 1.0 1.0))
        (Transformation|SetRelativeRotation _scene (Math|Rotator|MakeRotator (.roll _relativerotation) _pitch (.yaw _relativerotation)) false false))
      (:Eat
        (for _array_element (Collision|GetOverlappingActors (Variables|Default|GetEatBox) "/Game/GameObjects/TumbleWeed_BP.TumbleWeed_BP_C" :!class /Script/Engine.PrimitiveComponent)
          (bind _astumble_weed_bp (Utilities|Casting|CastToTumbleWeed_BP _array_element))
          (Default|Kill _astumble_weed_bp))))))

(event Custom|StopWalk
  (bind _scene (Variables|Default|GetScene))
  (bind _scene_2 (Variables|Default|GetScene))
  (bind _relativerotation (Variables|/Script/Engine.SceneComponent|GetRelativeRotation _scene_2))
  (bind _relativerotation_2 (Variables|/Script/Engine.SceneComponent|GetRelativeRotation _scene))
  (Utilities|FlowControl|Sequence
    (:then_0
      (bind _roll (Timeline|Walk_timeline Stop)
        (:Update
          (Transformation|SetRelativeRotation _scene_2 (Math|Rotator|MakeRotator (* _roll 5.0) (.pitch _relativerotation) (.yaw _relativerotation)) false false))
        (:Steps
          (Audio|SpawnSoundatLocation "/Game/Audio/Cues/CowStep_Cue.CowStep_Cue" (Transformation|GetActorLocation) "0, 0, 0" 1.0 1.0 0.0 0 0))))
    (:then_1
      (Transformation|SetRelativeRotation _scene (Math|Rotator|MakeRotator 0.0 (.pitch _relativerotation_2) (.yaw _relativerotation_2)) false false))))

(event Custom|StartWalk
  (bind _scene (Variables|Default|GetScene))
  (bind _relativerotation (Variables|/Script/Engine.SceneComponent|GetRelativeRotation _scene))
  (bind _roll (Timeline|Walk_timeline Play)
    (:Update
      (Transformation|SetRelativeRotation _scene (Math|Rotator|MakeRotator (* _roll 5.0) (.pitch _relativerotation) (.yaw _relativerotation)) false false))
    (:Steps
      (Audio|SpawnSoundatLocation "/Game/Audio/Cues/CowStep_Cue.CowStep_Cue" (Transformation|GetActorLocation) "0, 0, 0" 1.0 1.0 0.0 0 0))))

(event Custom|Moo
  (Components|Timeline|SetPlayRate (Variables|Default|GetMoo_Timeline) (Math|Random|RandomFloatinRange 0.5 2.0))
  (Timeline|Moo_Timeline PlayFromStart
    (:Moo
      (Audio|SpawnSoundatLocation "/Game/Audio/Cues/CowMooh_Cue.CowMooh_Cue" (Transformation|GetActorLocation) "0, 0, 0" 1.0 1.0 0.0 0 0)
      (CallFunction|Moo))))

(event Custom|TestGoto
  (CallFunction|Goto (+ (Transformation|GetActorLocation) "0.000000,-15000.000000,0.000000")))

(event EventBeginPlay
  (|CallParentFunction)
  (Components|Timeline|SetPlayRate (Variables|Default|GetWalk_timeline) 1.5)
  (Variables|Default|SetInitialTransform (Transformation|GetActorTransform))
  (Class|TWABlueprintLibrary|RegisterResetable)
  (Utilities|FlowControl|Delay 3.0)
  (CallFunction|Moo))

(event EventReset
  (Transformation|SetActorTransform (Variables|Default|GetInitialTransform))
  (CallFunction|SetGoto false)
  (Variables|Default|SetGotoStuckDuration -1.0)
  (Audio|Components|Audio|Stop (Variables|Default|GetMoo_Timeline))
  (Utilities|FlowControl|Delay 3.0)
  (CallFunction|Moo))

(event EventTick
  (params (DeltaSeconds :type Float%20%28single-precision%29))
  (CallFunction|TickGoto DeltaSeconds))

(event EventEndPlay
  (params (EndPlayReason :type EEndPlayReason%20Enum :default "Destroyed"))
  (|CallParentFunction EndPlayReason)
  (Class|TWABlueprintLibrary|UnregisterResetable))

(fn ConstructionScript)

(fn CheckforEat
  (bind _eatbox (Variables|Default|GetEatBox))
  (for _array_element (Collision|GetOverlappingActors _eatbox "/Game/GameObjects/TumbleWeed_BP.TumbleWeed_BP_C" :!class /Script/Engine.PrimitiveComponent)
    (bind _astumble_weed_bp (Utilities|Casting|CastToTumbleWeed_BP _array_element))
    (if (not (Class|Flammable|IsFlaming _astumble_weed_bp))
      (Default|SetForcedLocation _astumble_weed_bp (Transformation|GetWorldLocation _eatbox))
      (CallFunction|Eat))))

(fn Goto
  (params (GotoLocation :type Vector))
  (Variables|Default|SetGotoLocation GotoLocation)
  (CallFunction|SetGoto true))

(fn SetGoto
  (params (bGoto :type Boolean))
  (bind _output_get (Variables|Default|SetbGoto bGoto))
  (if _output_get
    (CallFunction|StartWalk)
    (Variables|Default|SetGotoStuckDuration 0.0)
    (Variables|Default|SetGotoLastLocation (Transformation|GetActorLocation))
    (else
      (CallFunction|StopWalk))))

(fn TickGoto
  (params (DeltaTime :type Float%20%28single-precision%29))
  (bind _returnvalue (Transformation|GetActorLocation))
  (bind _returnvalue_2 (Transformation|GetActorLocation))
  (bind _gotospeed (Variables|Default|GetGotoSpeed))
  (bind _gotolocation (Variables|Default|GetGotoLocation))
  (bind _returnvalue_3 (Math|Interpolation|VInterptoConstant _returnvalue_2 _gotolocation DeltaTime _gotospeed))
  (if (Variables|Default|GetbGoto)
    (bind _output_get (LocalVariables|SetInterpGoto _returnvalue_3))
    (Transformation|SetActorLocation _returnvalue_3 true false)
    (if (Math|Vector|VectorIsNearlyZero (- _output_get _gotolocation))
      ;[1 1 1] Done
      (CallFunction|SetGoto false)
      (elif (Math|Vector|VectorIsNearlyZero (- _returnvalue (Variables|Default|GetGotoLastLocation)))
        (bind _output_get_2 (Variables|Default|SetGotoStuckDuration (+ (Variables|Default|GetGotoStuckDuration) DeltaTime)))
        (if (> _output_get_2 1.0)
          ;[1 1 1] Stuck
          (CallFunction|SetGoto false))
        (else
          (Variables|Default|SetGotoLastLocation _returnvalue)
          (Variables|Default|SetGotoStuckDuration 0.0))))))

(fn CheckforSense
  (bind _returnvalue (Transformation|GetActorLocation))
  (bind _returnvalue_2 (Transformation|GetActorForwardVector))
  (for _array_element (Collision|GetOverlappingActors (Variables|Default|GetSenseBox) 0 :!class /Script/Engine.PrimitiveComponent)
    (if (Utilities|DoesObjectImplementInterface _array_element "/Script/GGJ.Flammable")
      (bind _returnvalue_3 (Class|Flammable|IsFlaming(Message) _array_element))
      (if _returnvalue_3
        (CallFunction|Goto (+ _returnvalue (* _returnvalue_2 (Math|Float|Sign(Float) (Math|Vector|DotProduct (- (Transformation|GetActorLocation _array_element) _returnvalue) _returnvalue_2)) -1.5e+02)))))))