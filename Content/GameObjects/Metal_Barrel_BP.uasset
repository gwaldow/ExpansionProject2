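; Metal barrel physics prop that responds to wind and supports level-style resets.
; It registers as windable and resetable, restores its starting transform and kills velocity on reset, and calls RegisterWindable again in EndPlay.
; Wind only pushes it when lying near horizontal, scaled by the cubed dot product with its sideways rolling direction and applied through clamped SimplePhysicsWind.
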(event EventBeginPlay
  (|CallParentFunction)
  (Class|TWABlueprintLibrary|RegisterWindable)
  (Class|TWABlueprintLibrary|RegisterResetable)
  (Variables|Default|SetInitialTransform (Transformation|GetActorTransform)))

(event EventWind
  (params (windForce :type Vector%20%28by%20ref%29 :default "0, 0, 0"))
  (if (< (Math|Float|Absolute(Float) (.z (Math|Vector|GetUpVector (Variables|Default|GetMesh)))) 0.35)
    (Class|TWABlueprintLibrary|SimplePhysicsWind 0 (* windForce 4.0 (Math|Float|Power (Math|Float|Absolute(Float) (Math|Vector|DotProduct windForce (Math|Vector|CrossProduct (Math|Vector|GetUpVector (Variables|Default|GetMesh)) "0.000000,0.000000,1.000000"))) 3.0)) 3.0)))

(event EventReset
  (Transformation|SetActorTransform (Variables|Default|GetInitialTransform))
  (Class|TWABlueprintLibrary|KillVelocity self))

(event EventEndPlay
  (params (EndPlayReason :type EEndPlayReason%20Enum :default "Destroyed"))
  (|CallParentFunction EndPlayReason)
  (Class|TWABlueprintLibrary|RegisterWindable)
  (Class|TWABlueprintLibrary|UnregisterResetable))

(fn ConstructionScript)

(fn GetZLimit
  (return ""))