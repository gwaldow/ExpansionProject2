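; Tumbleweed actor that is pushed by wind physics and can catch fire, burning away over a set duration.
; SetOnFire toggles the particles, status widget and a runtime fire component, then notifies the player pawn.
; Tick grows the flame and progress until burnout destroys the actor, and can interpolate it toward a forced location.
; Each tick it also makes every Cow_BP run eat and sense checks.
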(event Custom|Kill
  (Actor|DestroyActor))

(event EventBeginPlay
  (bind _returnvalue (Class|TWABlueprintLibrary|GetLocalPawn))
  (|CallParentFunction)
  (Class|TWABlueprintLibrary|RegisterWindable)
  (Utilities|IsValid _returnvalue
    (:Is%20Valid
      (Class|TWAPawn|RecomputeViewTargets _returnvalue))))

(event EventWind
  (params (windForce :type Vector%20%28by%20ref%29 :default "0, 0, 0"))
  (Class|TWABlueprintLibrary|SimplePhysicsWind 0 windForce -1.0))

(event EventCatchFire
  (CallFunction|SetonFire true))

(event EventEndPlay
  (params (EndPlayReason :type EEndPlayReason%20Enum :default "Destroyed"))
  (bind _returnvalue (Class|TWABlueprintLibrary|GetLocalPawn))
  (|CallParentFunction EndPlayReason)
  (Class|TWABlueprintLibrary|UnregisterWindable)
  (Utilities|IsValid _returnvalue
    (:Is%20Valid
      (Class|TWAPawn|RecomputeViewTargets _returnvalue))))

(event EventTick
  (params (DeltaSeconds :type Float%20%28single-precision%29))
  (CallFunction|TickonFire DeltaSeconds)
  (CallFunction|TickForcedLocation DeltaSeconds))

(event EventExtinguish
  (CallFunction|SetonFire false))

(fn ConstructionScript)

(fn SetonFire
  (params (OnFire :type Boolean))
  (bind _returnvalue (Actor|GetComponentbyClass "/Script/GGJ.FireComponent"))
  (bind _p_fire (Variables|Default|GetP_Fire))
  (bind _statuswidget (Variables|Default|GetStatusWidget))
  (bind _returnvalue_2 (UserInterface|GetWidget _statuswidget))
  (bind _astumble_weed_status (Utilities|Casting|CastToTumbleWeedStatus _returnvalue_2))
  (Utilities|FlowControl|Sequence
    (:then_0
      (bind _output_get (Variables|Default|SetOnFire OnFire))
      (if _output_get
        (Components|Activation|Activate _p_fire false)
        (CallFunction|RefreshFireScale)
        (Default|SetIcon _astumble_weed_status "NewEnumerator1")
        (Utilities|IsValid (Actor|GetComponentbyClass "/Script/GGJ.FireComponent")
          (:Is%20Not%20Valid
            (bind _returnvalue_3 (Game|AddComponentbyClass "/Script/GGJ.FireComponent"))
            (Class|FireComponent|DelegateComponentHit _returnvalue_3 (Variables|Default|GetSphere))))
        (else
          (Components|Activation|Deactivate _p_fire)
          (Variables|Default|SetBurnedDuration 0.0)
          (Default|SetIcon _astumble_weed_status "NewEnumerator0")
          (Default|SetProgress _astumble_weed_status 0.0)
          (Utilities|IsValid _returnvalue
            (:Is%20Valid
              (Components|DestroyComponent _returnvalue))))))
    (:then_1
      (bind _astwapawn (Utilities|Casting|CastToTWAPawn (Game|Player|GetPlayerPawn 0)))
      (Class|TWAPawn|OnFireStateChanged _astwapawn))))

(fn RefreshFireScale
  (bind _output_get (LocalVariables|SetScale (Math|Float|MapRangeClamped (Variables|Default|GetBurnedDuration) 0.0 (Variables|Default|GetBurningDuration) 0.05 1.0)))
  (Transformation|SetWorldScale3D (Variables|Default|GetP_Fire) (Math|Vector|MakeVector _output_get _output_get _output_get))
  (Transformation|SetWorldLocationAndRotation (Variables|Default|GetP_Fire) (+ (Transformation|GetActorLocation) "0.000000,0.000000,35.000000") "0, 0, 0" false false))

(fn TickonFire
  (params (deltaTime :type Float%20%28double-precision%29))
  (bind _p_fire (Variables|Default|GetP_Fire))
  (Utilities|FlowControl|Sequence
    (:then_0
      (CallFunction|RefreshFireScale)
      (if (Variables|Default|GetOnFire)
        (bind _output_get (Variables|Default|SetBurnedDuration (+ deltaTime (Variables|Default|GetBurnedDuration))))
        (Default|SetProgress (.AsTumble%20Weed%20Status (Utilities|Casting|CastToTumbleWeedStatus (UserInterface|GetWidget (Variables|Default|GetStatusWidget)))) (/ _output_get (Variables|Default|GetBurningDuration)))
        (if (>= (/ _output_get (Variables|Default|GetBurningDuration)) 1.0)
          (Components|Activation|Deactivate _p_fire)
          (Effects|SpawnEmitteratLocation "/Game/StarterContent/Particles/P_FireFinished.P_FireFinished" (Transformation|GetWorldLocation _p_fire) "0, 0, 0" "1.000000,1.000000,1.000000" true "AutoRelease")
          (CallFunction|Kill))))
    (:then_1
      (bind _outactors (Actor|GetAllActorsOfClass "/Game/GameObjects/Cow_BP.Cow_BP_C"))
      (for _array_element _outactors
        (Default|CheckforEat _array_element)
        (Default|CheckforSense _array_element)))))

(fn TickForcedLocation
  (params (deltaTime :type Float%20%28double-precision%29))
  (if (Variables|Default|GetbForceToLocation)
    (Transformation|SetActorLocation (Math|Interpolation|VInterpTo (Transformation|GetActorLocation) (Variables|Default|GetForcedLocation) deltaTime 5e+01) false false)))

(fn SetForcedLocation
  (params (ForcedLocation :type Vector))
  (Variables|Default|SetbForceToLocation true)
  (Variables|Default|SetForcedLocation ForcedLocation))

(fn GetZLimit
  (return ""))

(fn IsFlaming
  (bind _returnvalue (Class|TWABlueprintLibrary|DefaultIsFlaming))
  (return (or _returnvalue (Variables|Default|GetOnFire))))