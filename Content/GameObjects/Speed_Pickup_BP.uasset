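; Speed pickup actor that triggers a speed-doubling effect when a TumbleWeed_BP overlaps it, then destroys itself.
; BeginPlay stores the start location and binds the overlap handler, which calls DoubleMySpeed.
; Tick spins the actor in yaw and sets its height from the start Z plus a scaled sine.
; The sine takes frame delta rather than elapsed time, so the offset follows frame time instead of oscillating.
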(event Custom|OnActorBeginOverlap_Event
  (params (OverlappedActor :type Actor%20Object%20Reference) (OtherActor :type Actor%20Object%20Reference))
  (Utilities|Casting|CastToTumbleWeed_BP OtherActor)
  (Default|CallDoubleMySpeed)
  (Actor|DestroyActor))

(event EventBeginPlay
  (Variables|Default|Setstartloc (Transformation|GetActorLocation))
  (EventDispatchers|AssignOnActorBeginOverlap (delegate Custom|OnActorBeginOverlap_Event)))

(event Collision|EventActorBeginOverlap
  (params (OtherActor :type Actor%20Object%20Reference)))

(event EventTick
  (params (DeltaSeconds :type Float%20%28single-precision%29))
  (Class|Actor|AddActorWorldRotation (Math|Rotator|MakeRotator 0.0 0.0 (Variables|Default|Getspinrate)))
  (Transformation|SetActorLocation (Math|Vector|MakeVector 0.0 0.0 (+ (.z (Variables|Default|Getstartloc)) (* (Math|Trig|Sin(Radians) DeltaSeconds) (Variables|Default|Getbobheight)))) false false))

(fn ConstructionScript)