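; Bird actor that hunts tumbleweeds by diving from its spline path and killing any it hits.
; While not diving, it sphere-traces downward each tick; spotting a tumbleweed pauses MySpline movement after a short delay and starts a dive.
; The dive follows a half sine wave straight down and back up over DiveDuration, rotates the bird along its motion, then resumes spline movement.
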(event EventBeginPlay)

(event EventTick
  (params (DeltaSeconds :type Float%20%28single-precision%29))
  (bind _returnvalue (Transformation|GetActorLocation))
  (bind _returnvalue_2 (Transformation|GetActorLocation))
  (bind _returnvalue_3 (Transformation|GetActorLocation))
  (if (Variables|Default|Getdiving)
    (bind _output_get (Variables|Default|SetDiveTime (+ (Variables|Default|GetDiveTime) DeltaSeconds)))
    (if (>= (* _output_get (/ (Math|Trig|GetPI) (Variables|Default|GetDiveDuration))) 3.14)
      (Default|StartMove (Variables|Default|GetMySpline))
      (Variables|Default|Setdiving false)
      (else
        (Transformation|SetActorLocation (Math|Vector|Lerp(Vector) (Variables|Default|GetStartDiveLoc) (- (Variables|Default|GetStartDiveLoc) "0.000000,0.000000,1000.000000") (Math|Trig|Sin(Radians) (* _output_get (/ (Math|Trig|GetPI) (Variables|Default|GetDiveDuration))))) false false)
        (Transformation|SetActorRotation (Math|Rotator|MakeRotfromX (- _returnvalue_2 (Variables|Default|GetPrevLocation))))
        (Variables|Default|SetPrevLocation _returnvalue_2)))
    (else
      (bind _outhits (Collision|MultiSphereTraceForObjects _returnvalue_3 (- _returnvalue_3 "0.000000,0.000000,1000.000000") 1e+02 (Variables|Default|GetSweepTypes) false 0 "None"))
      (for _array_element _outhits
        (Utilities|Casting|CastToTumbleWeed_BP (.hitactor _array_element))
        (Utilities|FlowControl|Delay 0.3)
        (Default|PauseMove (Variables|Default|GetMySpline))
        (Variables|Default|SetDiveTime DeltaSeconds)
        (Variables|Default|SetStartDiveLoc _returnvalue)
        (Variables|Default|Setdiving true)
        (Variables|Default|SetPrevLocation _returnvalue)))))

(event Collision|EventHit
  (params (MyComp :type Primitive%20Component%20Object%20Reference) (Other :type Actor%20Object%20Reference) (OtherComp :type Primitive%20Component%20Object%20Reference) (bSelfMoved :type Boolean) (HitLocation :type Vector :default "0, 0, 0") (HitNormal :type Vector :default "0, 0, 0") (NormalImpulse :type Vector :default "0, 0, 0") (Hit :type Hit%20Result%20Structure%20%28by%20ref%29))
  (bind _astumble_weed_bp (Utilities|Casting|CastToTumbleWeed_BP Other))
  (Default|Kill _astumble_weed_bp))

(fn ConstructionScript)