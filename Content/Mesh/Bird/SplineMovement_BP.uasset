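; Spline mover, stored with the Bird assets, that carries a referenced actor along a spline path in an endless loop.
; The construction script snaps the actor to the first spline point.
; From BeginPlay, a timeline with play rate scaled by TimelineLength maps its track to spline distance, setting location and tangent-facing rotation each update.
; When the timeline finishes, it restarts from the beginning.
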(event Custom|PlayTimeline
  (bind _spline (Variables|Default|GetSpline))
  (bind _actor (Variables|Default|GetActor))
  (bind _newtrack_0 (Timeline|Timeline PlayFromStart)
    (:Update
      (Transformation|SetActorLocation _actor (Spline|GetLocationatDistanceAlongSpline _spline (Math|Float|Lerp 0.0 (Spline|GetDistanceAlongSplineatSplinePoint (Variables|Default|GetSpline) (- (Spline|GetNumberOfSplinePoints (Variables|Default|GetSpline)) 1)) _newtrack_0) "World") false false)
      (Transformation|SetActorRotation _actor (Math|Conversions|RotationFromXVector (Spline|GetTangentatDistanceAlongSpline _spline (Math|Float|Lerp 0.0 (Spline|GetDistanceAlongSplineatSplinePoint (Variables|Default|GetSpline) (- (Spline|GetNumberOfSplinePoints (Variables|Default|GetSpline)) 1)) _newtrack_0) "World"))))
    (:Finished
      (CallFunction|PlayTimeline))))

(event EventBeginPlay
  (Components|Timeline|SetPlayRate (Variables|Default|GetTimeline) (/ 1.0 (Variables|Default|GetTimelineLength)))
  (CallFunction|PlayTimeline))

(fn ConstructionScript
  (Transformation|SetActorLocation (Variables|Default|GetActor) (Spline|GetLocationatSplinePoint (Variables|Default|GetSpline) 0 "World") false false))