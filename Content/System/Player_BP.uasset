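; Player Blueprint that adds screen-fade, wind visual and checkpoint audio feedback to the player.
; On BeginPlay it creates a fade widget, whose flag is toggled by death and respawn events.
; With a valid local controller, Tick feeds wind input to a VFX component: angle sets facing while input is non-zero, magnitude scales spawn rate.
; Reaching a checkpoint plays a 2D success sound.
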(event EventBeginPlay
  (bind _returnvalue (UserInterface|CreateWidget "/Game/Widgets/HUD/FadeOutWidget.FadeOutWidget_C"))
  (bind _output_get (Variables|Default|SetFadeWidget _returnvalue))
  (UserInterface|Viewport|AddtoViewport _output_get 0))

(event EventOnDeathFadeOut
  (Variables|/Game/Widgets/HUD/FadeOutWidget.FadeOutWidget_C|SetbFadeOut (Variables|Default|GetFadeWidget) true))

(event EventOnPlayerRespawn
  (Variables|/Game/Widgets/HUD/FadeOutWidget.FadeOutWidget_C|SetbFadeOut (Variables|Default|GetFadeWidget) false))

(event EventTick
  (params (DeltaSeconds :type Float%20%28single-precision%29))
  (bind _windvfx (Variables|Default|GetWindVFX))
  (Utilities|IsValid (Class|TWABlueprintLibrary|GetLocalController)
    (:Is%20Valid
      (if (Math|Float|NearlyEqual(Float) (Math|Vector2D|Vector2DLength (Class|TWABlueprintLibrary|GetWindInput)) 0.0 0.001)
        _
        (else
          (Niagara|SetNiagaraVariable(Vector3) _windvfx "FacingVector" (Math|Rotator|GetRotationXVector (Math|Vector|RotatorfromAxisandAngle "0.000000,0.000000,1.000000" (Class|TWABlueprintLibrary|GetWindAngle))))))
      (Niagara|SetNiagaraVariable(Float) _windvfx "SpawnRate" (* (Math|Vector2D|Vector2DLength (Class|TWABlueprintLibrary|GetWindInput)) 1e+01)))))

(event EventOnCheckpointReached
  (Audio|PlaySound2D "/Game/Audio/Cues/Success_Cue.Success_Cue" 1.0 1.0 0.0 0 0))

(fn ConstructionScript)